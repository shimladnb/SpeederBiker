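; Speeder bike handlebars that pitch to follow the player's VR motion controllers and derive a throttle value for each hand.
; BeginPlay grabs both controllers from the first BP_SH_SpeederBikePawn found and stores a pawn's initial relative transform.
; Each Tick, AnimateBars1 computes look-at pitch from each bar to its controller, offset by that stored location.
; The negated pitch becomes that hand's throttle, and an offset version rotates the bar.
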(event EventBeginPlay
  (CallFunction|SetMotionControllerRef1)
  (CallFunction|SetInitialPawnRoot))

(event EventTick
  (params (DeltaSeconds :type Float%20%28single-precision%29))
  (Utilities|FlowControl|Sequence
    (:then_0
      (bind _throttleamount (CallFunction|AnimateBars1 (Variables|Default|GethandleBarR) (Variables|Default|GetrightMotionController)))
      (Variables|Default|SetrightHandThrottle _throttleamount))
    (:then_1
      (bind _throttleamount_2 (CallFunction|AnimateBars1 (Variables|Default|GethandleBarL) (Variables|Default|GetleftMotionController)))
      (Variables|Default|SetleftHandThrottle _throttleamount_2))))

(fn ConstructionScript)

(fn AddCounter
  (Variables|Default|Setcounter (+ (Variables|Default|Getcounter) 1.0)))

(fn SetMotionControllerRef1
  (bind _outactors (Actor|GetAllActorsOfClass "/Game/VirtualRealityBP/Blueprints/BP_SH_SpeederBikePawn.BP_SH_SpeederBikePawn_C"))
  (bind _output_get (Variables|Default|SetmotionControllerPawnReference (Utilities|Array|Get(acopy) _outactors)))
  (CallFunction|SetMotionControllers _output_get))

(fn AnimateBars1
  (params (handleBar :type Static%20Mesh%20Component%20Object%20Reference) (motionController :type Motion%20Controller%20Component%20Object%20Reference))
  (bind _returnvalue (Transformation|GetRelativeTransform motionController))
  (bind _initialpawnroot (Variables|Default|GetinitialPawnRoot))
  (bind _relativelocation (Variables|/Script/Engine.SceneComponent|GetRelativeLocation handleBar))
  (bind _location (Math|Transform|BreakTransform _returnvalue))
  (bind _returnvalue_2 (+ _location (.location _initialpawnroot)))
  (bind _returnvalue_3 (Math|Rotator|FindLookatRotation _relativelocation _returnvalue_2))
  (bind _pitch (Math|Rotator|BreakRotator _returnvalue_3))
  (bind _returnvalue_4 (* _pitch -1.0))
  (Transformation|SetRelativeRotation handleBar (Math|Rotator|MakeRotator 0.0 (- _returnvalue_4 -4e+01) 0.0) false false)
  (return _returnvalue_4))

(fn SetMotionControllers
  (params (NewParam :type BP%20SH%20Speeder%20Bike%20Pawn%20Object%20Reference))
  (Variables|Default|SetrightMotionController (Variables|/Game/VirtualRealityBP/Blueprints/BP_MotionController.BP_MotionController_C|GetMotionController (Variables|/Game/VirtualRealityBP/Blueprints/BP_SH_SpeederBikePawn.BP_SH_SpeederBikePawn_C|GetRightController NewParam)))
  (Variables|Default|SetleftMotionController (Variables|/Game/VirtualRealityBP/Blueprints/BP_MotionController.BP_MotionController_C|GetMotionController (Variables|/Game/VirtualRealityBP/Blueprints/BP_SH_SpeederBikePawn.BP_SH_SpeederBikePawn_C|GetLeftController NewParam))))

(fn SetInitialPawnRoot
  (Variables|Default|SetinitialPawnRoot (Transformation|GetRelativeTransform (Variables|Default|GetBP_SH_SpeederBikePawn))))