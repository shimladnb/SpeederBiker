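; VR hover speeder bike driven by physics forces on a merged bike body.
; Each tick, the average of both hand throttles from a child handlebar actor sets forward force, and their difference sets yaw torque.
; The rider's sideways headset offset sets roll torque, so leaning banks the bike.
; On BeginPlay it applies damping and initializes front and back auto-damping hover thrusters on the body; the middle thruster array is never initialized.
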(event EventBeginPlay
  (CallFunction|SetHandleBarsRef1)
  (CallFunction|SetHoverParams))

(event EventTick
  (params (DeltaSeconds :type Float%20%28single-precision%29))
  (CallFunction|SetAcceleration1)
  (CallFunction|SetRollandSteer)
  (CallFunction|SetHmdOffset1)
  (Physics|AddForce (Variables|Default|GetmergedBike) (* (Math|Vector|GetForwardVector (Variables|Default|GetmergedBike)) (Variables|Default|Getacceleration)) "None" false)
  (Class|PrimitiveComponent|AddTorqueinDegrees (Variables|Default|GetmergedBike) (* (Math|Vector|GetUpVector (Variables|Default|GetmergedBike)) (Variables|Default|Getsteer)) "None" false)
  (Class|PrimitiveComponent|AddTorqueinDegrees (Variables|Default|GetmergedBike) (* (Math|Vector|GetForwardVector (Variables|Default|GetmergedBike)) (Variables|Default|Getroll)) "None" false))

(fn ConstructionScript
  (CallFunction|SetThrusterArrays))

(fn SetAcceleration1
  (bind _handlebarsref (Variables|Default|GethandleBarsRef))
  (bind _righthandthrottle (Variables|/Game/Assets/speederBike/BP_SH_HandleBars.BP_SH_HandleBars_C|GetrightHandThrottle _handlebarsref))
  (bind _lefthandthrottle (Variables|/Game/Assets/speederBike/BP_SH_HandleBars.BP_SH_HandleBars_C|GetleftHandThrottle _handlebarsref))
  (bind _returnvalue (Math|Float|MapRangeClamped _lefthandthrottle 0.0 -6e+01 0.0 1.0))
  (bind _returnvalue_2 (Math|Float|MapRangeClamped _righthandthrottle 0.0 -6e+01 0.0 1.0))
  (Variables|Default|SetRight%20Hand%20Throttle _returnvalue_2)
  (Variables|Default|SetLeft%20Hand%20Throttle _returnvalue)
  (Variables|Default|Setacceleration (* (/ (+ _returnvalue_2 _returnvalue) 2.0) (* (Variables|HoverParams|GetmaxSpeed) 1e+06))))

(fn SetRollandSteer
  (bind _right_hand_throttle (Variables|Default|GetRight%20Hand%20Throttle))
  (bind _left_hand_throttle (Variables|Default|GetLeft%20Hand%20Throttle))
  (bind _returnvalue (Math|Vector|MakeVector _left_hand_throttle 0.0 0.0))
  (bind _returnvalue_2 (Math|Vector|MakeVector _right_hand_throttle 0.0 0.0))
  (bind _returnvalue_3 (Math|Vector|Distance2D(Vector) _returnvalue_2 _returnvalue))
  (Variables|Default|Setsteer (* (+ (* _returnvalue_3 (* _right_hand_throttle -1.0)) (* _returnvalue_3 (* _left_hand_throttle 1.0))) (* (Variables|HoverParams|GetsteerMax) 1e+06)))
  (Variables|Default|Setroll (* (Variables|Default|GethmdOffset) (* (Variables|HoverParams|GetmaxRoll) 1e+06))))

(fn SetHandleBarsRef1
  (bind _asbp_sh_handle_bars (Utilities|Casting|CastToBP_SH_HandleBars (Variables|/Script/Engine.ChildActorComponent|GetChildActor (Variables|Default|GetBP_SH_HandleBars))))
  (Variables|Default|SethandleBarsRef _asbp_sh_handle_bars))

(fn SetHmdOffset1
  (Variables|Default|SethmdOffset (* (.Y (Math|Vector|BreakVector (.OutPosition (Class|SteamVRFunctionLibrary|GetTrackedDevicePositionandOrientation)))) -1.0)))

(fn SetHoverParams
  (Class|PrimitiveComponent|SetAngularDamping (Variables|Default|GetmergedBike) (Variables|HoverParams|GetangularDampening))
  (Class|PrimitiveComponent|SetLinearDamping (Variables|Default|GetmergedBike) (Variables|HoverParams|GetlinearDampening))
  (CallFunction|SetThrusterParams (Variables|Default|GetfrontThrustersArray))
  (CallFunction|SetThrusterParams (Variables|Default|GetbackThrustersArray)))

(fn SetThrusterArrays
  (Variables|Default|SetfrontThrustersArray (Utilities|Array|MakeArray (Variables|Default|GetBP_SH_HoverThrusterAutoDamp1) (Variables|Default|GetBP_SH_HoverThrusterAutoDamp0)))
  (Variables|Default|SetmidThrustersArray (Utilities|Array|MakeArray 0 0))
  (Variables|Default|SetbackThrustersArray (Utilities|Array|MakeArray (Variables|Default|GetBP_SH_HoverThrusterAutoDamp5) (Variables|Default|GetBP_SH_HoverThrusterAutoDamp4))))

(fn SetThrusterParams
  (params (Array :type Array%20of%20BP%20SH%20Hover%20Thruster%20Auto%20Damp%20Object%20References))
  (for _array_element Array
    (Default|InitComponent _array_element (Variables|Default|GetmergedBike))))