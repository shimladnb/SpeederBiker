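; Scatters low-poly trees on the surface within a scalable box area, built in the construction script.
; AmountOfTrees drives a loop that picks random points in the Box bounds and passes them to AddTree.
; AddTree line-traces vertically on Visibility, then places a new static mesh component at the hit location with random yaw and uniform scale.
; Randomness is unseeded, so each construction re-rolls the layout, and trace misses are not checked.
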(event EventBeginPlay)

(fn ConstructionScript
  (bind _box (Variables|Default|GetBox))
  (bind (_origin _boxextent) (Collision|GetComponentBounds _box))
  (Transformation|SetWorldScale3D (Variables|Default|GetBox) (Variables|Default|GetspawnBoxScale))
  (for _index (range 0 (Variables|Default|GetamountOfTrees))
    (CallFunction|AddTree "/Game/Geometry/Meshes/lowPolyTree.lowPolyTree" (Math|Random|RandomPointinBoundingBox _origin _boxextent))))

(fn AddTree
  (params (mesh :type Static%20Mesh%20Object%20Reference) (location :type Vector))
  (LocalVariables|SetlocalStaticMesh mesh)
  (bind _outhit (Collision|LineTraceByChannel (+ location "0, 0,99999.000000") (+ location "0, 0,-999999.000000") "TraceTypeQuery1" false 0 "None"))
  (bind _returnvalue (AddComponent|AddStaticMeshComponent false (Math|Transform|MakeTransform "0, 0, 0" (Math|Rotator|MakeRotator 0.0 0.0 (Math|Random|RandomFloatinRange -1.8e+02 1.8e+02)) (Math|Conversions|ToVector(Float) (Math|Random|RandomFloatinRange 0.9 1.5)))))
  (bind _output_get (LocalVariables|SetlocalStaticMeshComponent _returnvalue))
  (Components|StaticMesh|SetStaticMesh _output_get (LocalVariables|GetlocalStaticMesh))
  (Transformation|SetWorldLocation (LocalVariables|GetlocalStaticMeshComponent) (.location _outhit) false false))