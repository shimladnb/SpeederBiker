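; Third-person hover speeder bike, driven by applying physics forces to the MergedBike body.
; Construction groups auto-damping hover thruster components into arrays; BeginPlay sets body damping and initializes the front and back thrusters on that body.
; MoveForward adds force along the bike's forward vector, and MoveRight adds yaw torque around its up vector.
; Handlebar-throttle and HMD-offset functions exist but are not called in this graph.
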(event EventBeginPlay
  (CallFunction|SetHoverParams))

(event Input|AxisEvents|InputAxisMoveForward
  (params (AxisValue :type Float%20%28single-precision%29))
  (Physics|AddForce (Variables|Default|GetmergedBike) (* (Math|Vector|GetForwardVector (Variables|Default|GetmergedBike)) (* AxisValue (Variables|Default|Getacceleration))) "None" false))

(event Input|AxisEvents|InputAxisMoveRight
  (params (AxisValue :type Float%20%28single-precision%29))
  (Class|PrimitiveComponent|AddTorqueinDegrees (Variables|Default|GetmergedBike) (* (Math|Vector|GetUpVector (Variables|Default|GetmergedBike)) (* AxisValue (* (Variables|Default|Getsteer) -1.0))) "None" false))

(fn ConstructionScript
  (CallFunction|SetThrusterArrays))

(fn SetAcceleration1
  (bind _handlebarsref (Variables|Default|GethandleBarsRef))
  (bind _righthandthrottle (Variables|/Game/Assets/speederBike/BP_SH_HandleBars.BP_SH_HandleBars_C|GetrightHandThrottle _handlebarsref))
  (bind _lefthandthrottle (Variables|/Game/Assets/speederBike/BP_SH_HandleBars.BP_SH_HandleBars_C|GetleftHandThrottle _handlebarsref))
  (bind _returnvalue (Math|Float|MapRangeClamped _lefthandthrottle 0.0 -6e+01 0.0 1.0))
  (bind _returnvalue_2 (Math|Float|MapRangeClamped _righthandthrottle 0.0 -6e+01 0.0 1.0))
  (Variables|Default|SetRight%20Hand%20Throttle _returnvalue_2)
  (Variables|Default|SetLeft%20Hand%20Throttle _returnvalue)
  (Variables|Default|Setacceleration (* (/ (+ _returnvalue_2 _returnvalue) 2.0) (* (Variables|HoverParams|GetmaxSpeed) 1e+06))))

(fn SetHandleBarsRef1)

(fn SetHmdOffset1
  (Variables|Default|SethmdOffset (* (.Y (Math|Vector|BreakVector (.OutPosition (Class|SteamVRFunctionLibrary|GetTrackedDevicePositionandOrientation)))) -1.0)))

(fn SetHoverParams
  (Class|PrimitiveComponent|SetAngularDamping (Variables|Default|GetmergedBike) (Variables|HoverParams|GetangularDampening))
  (Class|PrimitiveComponent|SetLinearDamping (Variables|Default|GetmergedBike) (Variables|HoverParams|GetlinearDampening))
  (CallFunction|SetThrusterParams (Variables|Default|GetfrontThrustersArray))
  (CallFunction|SetThrusterParams (Variables|Default|GetbackThrustersArray)))

(fn SetThrusterArrays
  (Variables|Default|SetfrontThrustersArray (Utilities|Array|MakeArray (Variables|Default|GetBP_SH_HoverThrusterAutoDamp1) (Variables|Default|GetBP_SH_HoverThrusterAutoDamp0)))
  (Variables|Default|SetmidThrustersArray (Utilities|Array|MakeArray 0 0))
  (Variables|Default|SetbackThrustersArray (Utilities|Array|MakeArray (Variables|Default|GetBP_SH_HoverThrusterAutoDamp5) (Variables|Default|GetBP_SH_HoverThrusterAutoDamp4))))

(fn SetThrusterParams
  (params (Array :type Array%20of%20BP%20SH%20Hover%20Thruster%20Auto%20Damp%20Object%20References))
  (for _array_element Array
    (Default|InitComponent _array_element (Variables|Default|GetmergedBike))))