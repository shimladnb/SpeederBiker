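; BP_Hover is a player-driven hovercraft pawn suspended on four spring components that share its damping, length and stiffness settings.
; BeginPlay sets spring force from StartEngine, while movement inputs push the mesh along control-yaw axes, with strafing at half force.
; With the engine on, a one-shot timeline swings the camera behind the craft, then mesh yaw eases toward the camera.
; The engine toggle and runtime spring spawning are unwired.
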(event Custom|PlayTurnAnim
  (Utilities|FlowControl|DoOnce false
    (:Completed
      (Variables|/Script/Engine.SpringArmComponent|SetbUsePawnControlRotation (Variables|Default|GetSpringArm) false)
      (Pawn|SetControlRotation (Game|GetPlayerController 0) (Math|Rotator|MakeRotator 0.0 0.0 (.yaw (Transformation|GetWorldRotation (Variables|Default|GetMesh)))))
      (bind _alpha (Timeline|CameraTurnAnim PlayFromStart)
        (:Update
          (Variables|Default|SetTurnAlpha _alpha)
          (Transformation|SetWorldRotation (Variables|Default|GetSpringArm) (Math|Rotator|Lerp(Rotator) (Transformation|GetWorldRotation (Variables|Default|GetCamera)) (Transformation|GetWorldRotation (Variables|Default|GetMesh)) (Variables|Default|GetTurnAlpha)) false false))
        (:Finished
          (Variables|/Script/Engine.SpringArmComponent|SetbUsePawnControlRotation (Variables|Default|GetSpringArm) true)
          (Variables|Default|SetbCameraTurnFinished_? true)
          (Utilities|FlowControl|DoOnce false) ; enters at Reset
        )))))

(event Custom|ResetTurnAnim
  (Utilities|FlowControl|DoOnce false
    (:Completed
      (Variables|Default|SetbCameraTurnFinished_? false)
      (Utilities|FlowControl|DoOnce false) ; enters at Reset
    )))

(event EventBeginPlay
  (Variables|Default|SetSpringList (Utilities|Array|MakeArray (Variables|Default|GetBP_SpringComponent1) (Variables|Default|GetBP_SpringComponent2) (Variables|Default|GetBP_SpringComponent3) (Variables|Default|GetBP_SpringComponent)))
  (CallFunction|SetSpringParameters)
  (for _array_element (Variables|Default|GetSpringList)
    (Default|AdjustForce _array_element (Math|Float|SelectFloat 1.0 0.0 (Variables|Default|GetbStartEngine_?)))))

(event EventTick
  (params (DeltaSeconds :type Float%20%28single-precision%29))
  (bind _mesh (Variables|Default|GetMesh))
  (bind _returnvalue (Transformation|GetWorldRotation _mesh))
  (bind (_roll _pitch) (Math|Rotator|BreakRotator _returnvalue))
  (if (Variables|Default|GetbStartEngine_?)
    (if (not (Variables|Default|GetbCameraTurnFinished_?))
      (CallFunction|PlayTurnAnim)
      (else
        (Transformation|SetWorldRotation (Variables|Default|GetMesh) (Math|Rotator|MakeRotator _roll _pitch (.yaw (Math|Interpolation|RInterpTo _returnvalue (Transformation|GetWorldRotation (Variables|Default|GetCamera)) (Utilities|Time|GetWorldDeltaSeconds) 6.0))) false false)))
    (else
      (CallFunction|ResetTurnAnim))))

(event Input|AxisEvents|InputAxisLookUp
  (params (AxisValue :type Float%20%28single-precision%29))
  (Pawn|Input|AddControllerPitchInput AxisValue))

(event Input|AxisEvents|InputAxisTurn
  (params (AxisValue :type Float%20%28single-precision%29))
  (Pawn|Input|AddControllerYawInput AxisValue))

(event Input|AxisEvents|InputAxisMoveForward
  (params (AxisValue :type Float%20%28single-precision%29))
  (Physics|AddForce (Variables|Default|GetMesh) (* (* (Math|Vector|GetForwardVector (Math|Rotator|MakeRotator 0.0 0.0 (.yaw (Pawn|GetControlRotation :!class /Script/Engine.Pawn)))) AxisValue) (Variables|Default|GetForceToAdd)) "None" false))

(event Input|AxisEvents|InputAxisMoveRight
  (params (AxisValue :type Float%20%28single-precision%29))
  (Physics|AddForce (Variables|Default|GetMesh) (* (* (Math|Vector|GetRightVector (Math|Rotator|MakeRotator 0.0 0.0 (.yaw (Pawn|GetControlRotation :!class /Script/Engine.Pawn)))) AxisValue) (/ (Variables|Default|GetForceToAdd) 2.0)) "None" false))

(fn ConstructionScript)

(fn CalculateSpringOffset
  (bind _mesh (Variables|Default|GetMesh))
  (bind (_origin _boxextent) (Collision|GetComponentBounds _mesh))
  (LocalVariables|SetOrigin _origin)
  (LocalVariables|SetBounds _boxextent)
  (LocalVariables|SetBottomLine (.z (LocalVariables|GetOrigin)))
  (return (Utilities|Array|MakeArray (Math|Vector|MakeVector (- (.x (LocalVariables|GetOrigin)) (.x (LocalVariables|GetBounds))) (- (.y (LocalVariables|GetOrigin)) (.y (LocalVariables|GetBounds))) (LocalVariables|GetBottomLine)) (Math|Vector|MakeVector (+ (.x (LocalVariables|GetOrigin)) (.x (LocalVariables|GetBounds))) (- (.y (LocalVariables|GetOrigin)) (.y (LocalVariables|GetBounds))) (LocalVariables|GetBottomLine)) (Math|Vector|MakeVector (+ (.x (LocalVariables|GetOrigin)) (.x (LocalVariables|GetBounds))) (+ (.y (LocalVariables|GetOrigin)) (.y (LocalVariables|GetBounds))) (LocalVariables|GetBottomLine)) (Math|Vector|MakeVector (- (.x (LocalVariables|GetOrigin)) (.x (LocalVariables|GetBounds))) (+ (.y (LocalVariables|GetOrigin)) (.y (LocalVariables|GetBounds))) (LocalVariables|GetBottomLine)))))

(fn SetSpringParameters
  (for _array_element (Variables|Default|GetSpringList)
    (Variables|/Game/Assets/HoverCraftExample/BP_SpringComponent.BP_SpringComponent_C|SetDamping _array_element (Variables|hoverSprings|GetDamping))
    (Variables|/Game/Assets/HoverCraftExample/BP_SpringComponent.BP_SpringComponent_C|SetSpringLength _array_element (Variables|hoverSprings|GetSpring%20Length))
    (Variables|/Game/Assets/HoverCraftExample/BP_SpringComponent.BP_SpringComponent_C|SetStiffness _array_element (Variables|hoverSprings|GetStiffness))))