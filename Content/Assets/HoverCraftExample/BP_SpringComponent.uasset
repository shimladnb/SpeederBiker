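; Spring component for the hovercraft example that acts as one suspension point on the physics body it references as Daddy.
; Each tick it traces down its local up axis and applies a damped spring force along the hit normal, using compression and its rate of change.
; Without a hit it applies a fixed downward force at that point.
; AdjustForce sets the spring force multiplier, and zero disables all forces.
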(event EventTick
  (params (DeltaSeconds :type Float%20%28single-precision%29))
  (if (!= (Variables|Default|GetForceMod) 0.0)
    (Variables|Default|SetSpringLocation (Transformation|GetWorldLocation))
    (bind (_outhit _returnvalue) (Collision|LineTraceByChannel (Variables|Default|GetSpringLocation) (- (Variables|Default|GetSpringLocation) (* (Math|Vector|GetUpVector) (Variables|Default|GetSpringLength))) "TraceTypeQuery1" false 0 "ForOneFrame" true "(R=1.000000,G=0.000000,B=0.000000,A=1.000000)" "(R=0.000000,G=1.000000,B=0.000000,A=1.000000)" 1.0))
    (if _returnvalue
      (Class|PrimitiveComponent|AddForceatLocation (Variables|Default|Getdaddy) (CallFunction|CalculateSpringForce (.Distance (Collision|BreakHitResult _outhit)) (.Normal (Collision|BreakHitResult _outhit))) (Variables|Default|GetSpringLocation) "None")
      (Variables|Default|SetSuspensionPrevious (Variables|Default|GetSuspensionDelta))
      (else
        (Class|PrimitiveComponent|AddForceatLocation (Variables|Default|Getdaddy) (Math|Vector|MakeVector 0.0 0.0 -1.8e+05) (Variables|Default|GetSpringLocation) "None")))))

(fn CalculateSpringForce
  (params (Distance :type Float%20%28single-precision%29) (Normal :type Vector))
  (Variables|Default|SetSuspensionDelta (- (Variables|Default|GetSpringLength) Distance))
  (return (* Normal (* (+ (* (Variables|Default|GetSuspensionDelta) (Variables|Default|GetStiffness)) (* (/ (- (Variables|Default|GetSuspensionDelta) (Variables|Default|GetSuspensionPrevious)) (Utilities|Time|GetWorldDeltaSeconds)) (Variables|Default|GetDamping))) (Variables|Default|GetForceMod)))))

(fn AdjustForce
  (params (InForce :type Float%20%28single-precision%29))
  (Variables|Default|SetForceMod InForce))