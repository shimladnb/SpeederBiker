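; BP_SH_TestGun is a test gun for the hovercraft example that fires debug-drawn line traces from one of two fire points.
; Fire selects the fire point from a flag and calls TraceForward, ignoring the owner.
; TraceForward nudges the forward vector upward, clamps its Z so the shot never aims above horizontal, and traces an extremely long ray.
; It returns the hit, but Fire does nothing with it.
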(event EventBeginPlay)

(event Collision|EventActorBeginOverlap
  (params (OtherActor :type Actor%20Object%20Reference)))

(event EventTick
  (params (DeltaSeconds :type Float%20%28single-precision%29)))

(fn ConstructionScript)

(fn Fire
  (params (firePoint1 :type Boolean) (forwardVector :type Vector) (owner :type Actor%20Object%20Reference))
  (if firePoint1
    (CallFunction|TraceForward (Variables|Default|GetfirePoint1) forwardVector owner)
    (else
      (CallFunction|TraceForward (Variables|Default|GetfirePoint2) forwardVector owner))))

(fn TraceForward
  (params (firePoint :type Scene%20Component%20Object%20Reference) (forwardVector :type Vector) (ignoreOwner :type Actor%20Object%20Reference))
  (bind _returnvalue (Transformation|GetWorldLocation firePoint))
  (bind _returnvalue_2 (+ forwardVector "0, 0,0.200000"))
  (LocalVariables|SetlocalOwner ignoreOwner)
  (bind _outhit (Collision|LineTraceByChannel _returnvalue (+ _returnvalue (* (Math|Vector|MakeVector (.x _returnvalue_2) (.y _returnvalue_2) (Math|Float|Clamp(Float) (.z _returnvalue_2) -1.0 0.0)) 100000000376832.0)) "TraceTypeQuery3" false (Utilities|Array|MakeArray (LocalVariables|GetlocalOwner)) "ForDuration" true "(R=0.000000,G=1.000000,B=0.145541,A=1.000000)" "(R=1.000000,G=0.000000,B=0.538267,A=1.000000)"))
  (return _outhit))